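; Cuboid is an actor with a flattened static mesh that spins continuously while its red color value climbs.
; The construction script squashes the mesh height, and BeginPlay calls Func to set the starting rotation and color.
; Tick adds a fixed rotation and increments R each frame without delta-time scaling, writing R to the materials' Color parameter.
; The Click event resets R to zero, restarting the color ramp.
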(event `self.ReceiveBeginPlay`
  (`self.Func`))

(event `self.ReceiveTick`
  (params (DeltaSeconds :type "Float (single-precision)"))
  (`SceneComponent.K2_SetWorldRotation` (`self.StaticMeshComponent`) (`KismetMathLibrary.ComposeRotators` (`SceneComponent.K2_GetComponentRotation` (`self.StaticMeshComponent`)) (struct :`Yaw` 1.0)) false false)
  (set `self.R` (+ (`self.R`) 0.1))
  (`MeshComponent.SetVectorParameterValueOnMaterials` (`self.StaticMeshComponent`) "Color" (`KismetMathLibrary.MakeVector` (`self.R`))))

(event `ClickableInterface.Click`
  (set `self.R` 0.0))

(fn `Func`
  (bind _staticmeshcomponent (`self.StaticMeshComponent`))
  (`SceneComponent.K2_SetWorldRotation` _staticmeshcomponent (struct :`Yaw` 30.0) false false)
  (`MeshComponent.SetVectorParameterValueOnMaterials` _staticmeshcomponent "Color" (`KismetMathLibrary.MakeVector` (`self.R`))))

(fn `UserConstructionScript`
  (`SceneComponent.SetWorldScale3D` (`self.StaticMeshComponent`) (1.0 1.0 0.5)))