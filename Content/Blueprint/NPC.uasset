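; NPC character that wanders between random target points tagged "NPCNoob" and periodically jumps, reacting to a nearby VR player.
; Movement loop picks a random walk speed and point for AIMoveTo, pausing after arrival, while a parallel loop jumps after random delays.
; Capsule overlap with VRPawn redirects movement to the current location and sets IsPlayerClose, stopping both loops from repeating.
; Overlap end restarts both but never clears that flag.
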(event `self.ReceiveBeginPlay`
  (bind _outactors (`GameplayStatics.GetAllActorsOfClassWithTag` "/Script/Engine.TargetPoint" "NPCNoob"))
  (set `self.TargetPointList` _outactors)
  (`self.Movenment`)
  (`self.Jumping`))

(event `Jumping`
  (`KismetSystemLibrary.Delay` (`KismetMathLibrary.RandomFloatInRange` 3.0 8.0))
  (if (>= (`MovementComponent.GetMaxSpeed` (`self.CharacterMovement`)) 0.0)
    (`self.Jump`)
    (if (not (`self.IsPlayerClose`))
      (`self.Jumping`))))

(event `Movenment`
  (bind _output (`|GetArrayItem` (`self.TargetPointList`) (`KismetMathLibrary.RandomIntegerInRange` 0 (- (`KismetArrayLibrary.Array_Length` (`self.TargetPointList`)) 1))))
  (`/Engine/EditorBlueprintResources/StandardMacros.IsValid` _output
    (:`Is Valid`
      (set `CharacterMovementComponent.MaxWalkSpeed` (`KismetMathLibrary.RandomFloatInRange` 100.0 300.0) (`self.CharacterMovement`))
      (`|AIMoveTo` self (`self.K2_GetActorLocation`) _output
        (:`OnSuccess`
          (`KismetSystemLibrary.Delay` 5.0)
          (if (not (`self.IsPlayerClose`))
            (`self.Movenment`)))))))

(event `self.Capsule.OnComponentBeginOverlap`
  (params (OverlappedComponent :type "PrimitiveComponent Object Reference") (OtherActor :type "Actor Object Reference") (OtherComp :type "PrimitiveComponent Object Reference") (OtherBodyIndex :type Integer) (bFromSweep :type Boolean) (SweepResult :type "HitResult Structure (by ref)"))
  (cast `/Game/Blueprint/VRPawn` OtherActor)
  (`|AIMoveTo` self (`self.K2_GetActorLocation` self) null
    (:`then`
      (set `self.IsPlayerClose` true))))

(event `self.Capsule.OnComponentEndOverlap`
  (params (OverlappedComponent :type "PrimitiveComponent Object Reference") (OtherActor :type "Actor Object Reference") (OtherComp :type "PrimitiveComponent Object Reference") (OtherBodyIndex :type Integer))
  (cast `/Game/Blueprint/VRPawn` OtherActor)
  (`self.Jumping`)
  (`self.Movenment`))

(fn `UserConstructionScript`)