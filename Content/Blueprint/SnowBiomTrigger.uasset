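; Snow biome trigger volume that reskins pistols and cuboid pickables as they cross its Box boundary.
; On begin overlap, pistols call ChangeMatToSnow and cuboid pickables get the Pistol1_Inst material on slot 0.
; On end overlap, both switch to grass: pistols through ChangeMatToGrass, cuboids through Pistol1_Grass_Inst, with no record of their earlier material.
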(event `self.Box.OnComponentBeginOverlap`
  (params (OverlappedComponent :type "PrimitiveComponent Object Reference") (OtherActor :type "Actor Object Reference") (OtherComp :type "PrimitiveComponent Object Reference") (OtherBodyIndex :type Integer) (bFromSweep :type Boolean) (SweepResult :type "HitResult Structure (by ref)"))
  (`|ExecutionSequence`
    (:`then_0`
      (bind _aspistol (cast `Pistol` OtherActor))
      (`Pistol.ChangeMatToSnow` _aspistol))
    (:`then_1`
      (bind _ascuboid_pickable (cast `/Game/Blueprint/CuboidPickable` OtherActor))
      (`PrimitiveComponent.SetMaterial` (`BaseActor.StaticMeshComponent` _ascuboid_pickable) 0 "/Game/Materials/Pistol1_Inst.Pistol1_Inst"))))

(event `self.Box.OnComponentEndOverlap`
  (params (OverlappedComponent :type "PrimitiveComponent Object Reference") (OtherActor :type "Actor Object Reference") (OtherComp :type "PrimitiveComponent Object Reference") (OtherBodyIndex :type Integer))
  (`|ExecutionSequence`
    (:`then_0`
      (bind _aspistol (cast `Pistol` OtherActor))
      (`Pistol.ChangeMatToGrass` _aspistol))
    (:`then_1`
      (bind _ascuboid_pickable (cast `/Game/Blueprint/CuboidPickable` OtherActor))
      (`PrimitiveComponent.SetMaterial` (`BaseActor.StaticMeshComponent` _ascuboid_pickable) 0 "/Game/Materials/Pistol1_Grass_Inst.Pistol1_Grass_Inst"))))

(fn `UserConstructionScript`)